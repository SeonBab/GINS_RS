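; Skeletal mesh component Blueprint from a Niagara creature-summon effects pack that erodes its material over time and then destroys itself.
; On BeginPlay it makes a dynamic instance of the first material and reads its starting Erosion value.
; After a delay, a timed Delay loop, gated by Eroding, raises that parameter until it passes the target.
; A separate delayed event, started first, destroys the component independently of erosion progress.
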(event Custom|DelayToDestroyEvent
  (Utilities|FlowControl|Delay (Variables|Default|GetDelayToDestroy))
  (Components|DestroyComponent))

(event EventBeginPlay
  (CallFunction|DelaytoDestroyEvent)
  (bind _returnvalue (Rendering|Material|CreateDynamicMaterialInstance 0 (Rendering|Material|GetMaterial 0) "None" :!class /Script/Engine.PrimitiveComponent))
  (bind _returnvalue_2 (Rendering|Material|GetScalarParameterValue _returnvalue "Erosion" :!class /Script/Engine.MaterialInstanceDynamic))
  (Variables|Default|SetCurrentErosion _returnvalue_2)
  (Utilities|FlowControl|Delay (Variables|Default|GetDelayToErode))
  (if (Variables|Default|GetEroding) :!label _label
    (bind _output_get (Variables|Default|SetCurrentErosion (+ (Variables|Default|GetCurrentErosion) (Variables|Default|GetErodeRate))))
    (Rendering|Material|SetScalarParameterValue _returnvalue "Erosion" _output_get :!class /Script/Engine.MaterialInstanceDynamic)
    (Utilities|FlowControl|Delay (Variables|Default|GetRefreshRate))
    (if (<= (Variables|Default|GetCurrentErosion) (Variables|Default|GetErodeTarget))
      (goto _label)
      (else
        (Variables|Default|SetEroding false)))))

(event EventTick
  (params (DeltaSeconds :type Float%20%28single-precision%29)))