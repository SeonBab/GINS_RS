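; FollowGround is a scene component that keeps its owning actor snapped to the surface below it, in a summon-creatures Niagara effects pack.
; While FollowGround is enabled, each tick casts a Visibility line trace straight down from the component's location over LineTraceDistance.
; On a hit, it moves the owner to the hit point raised by OffsetFromGround, without sweeping; without a hit, the owner is left in place.
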(event EventTick
  (params (DeltaSeconds :type Float%20%28single-precision%29))
  (bind _returnvalue (Transformation|GetWorldLocation))
  (if (Variables|Default|GetFollowGround)
    (bind (_outhit _returnvalue_2) (Collision|LineTraceByChannel _returnvalue (+ _returnvalue (Math|Vector|MakeVector 0.0 0.0 (* (Variables|Default|GetLineTraceDistance) -1.0))) "TraceTypeQuery1" false 0 "None" true "(R=1.000000,G=0.000000,B=0.000000,A=1.000000)" "(R=0.000000,G=1.000000,B=0.000000,A=1.000000)" 0.0))
    (if _returnvalue_2
      (Transformation|SetActorLocation (Components|GetOwner) (+ (.location _outhit) (Math|Vector|MakeVector 0.0 0.0 (Variables|Default|GetOffsetFromGround))) false false))))