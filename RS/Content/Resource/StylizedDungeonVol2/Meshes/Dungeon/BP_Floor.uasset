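; BP_Floor is a construction-time dungeon floor piece that deforms meshes along an editable spline.
; The construction script sets two spline mesh components to the same start and end, using local positions and tangents from the first two points of the Ww spline.
; Only that single segment is covered, the Spline variable is unused, and the event graph has no active logic.
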(event EventBeginPlay)

(event Collision|EventActorBeginOverlap
  (params (OtherActor :type Actor%20Object%20Reference)))

(event EventTick
  (params (DeltaSeconds :type Float%20%28single-precision%29)))

(fn ConstructionScript
  (bind _ww (Variables|Default|Getww))
  (bind _ww_2 (Variables|Default|Getww))
  (SplineMesh|SetStartandEnd (Variables|Default|GetSplineMesh) (Spline|GetLocationatSplinePoint _ww_2 0 "Local") (Spline|GetTangentatSplinePoint _ww_2 0 "Local") (Spline|GetLocationatSplinePoint _ww_2 1 "Local") (Spline|GetTangentatSplinePoint _ww_2 1 "Local") true :!class /Script/Engine.SplineMeshComponent)
  (SplineMesh|SetStartandEnd (Variables|Default|GetSplineMesh1) (Spline|GetLocationatSplinePoint _ww 0 "Local") (Spline|GetTangentatSplinePoint _ww 0 "Local") (Spline|GetLocationatSplinePoint _ww 1 "Local") (Spline|GetTangentatSplinePoint _ww 1 "Local") true :!class /Script/Engine.SplineMeshComponent))