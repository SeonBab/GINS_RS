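; BP_Floor_1 is a dungeon floor Blueprint whose construction script shapes a SplineMesh using circle math driven by Radius and Count.
; Each loop pass puts the start position on the circle and the next point into the start tangent, while end position and end tangent share a tenth-radius vector.
; The loop creates no components and rewrites the same SplineMesh, so only the last pass persists.
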(event EventBeginPlay)

(event Collision|EventActorBeginOverlap
  (params (OtherActor :type Actor%20Object%20Reference)))

(event EventTick
  (params (DeltaSeconds :type Float%20%28single-precision%29)))

(fn ConstructionScript
  (bind _count (Variables|Default|GetCount))
  (bind _radius (Variables|Default|GetRadius))
  (bind _returnvalue (/ 360 _count))
  (bind _returnvalue_2 (* _radius 0.1))
  (for _index (range 0 (- (Variables|Default|GetCount) 1))
    (SplineMesh|SetStartandEnd (Variables|Default|GetSplineMesh) (Math|Vector|MakeVector (* (Variables|Default|GetRadius) (Math|Trig|Cos(Degrees) (Math|Conversions|ToFloat(Integer) (* _index _returnvalue)))) (* (Math|Trig|Sin(Degrees) (Math|Conversions|ToFloat(Integer) (* _index _returnvalue))) (Variables|Default|GetRadius)) 0.0) (Math|Vector|MakeVector (* (Variables|Default|GetRadius) (Math|Trig|Cos(Degrees) (Math|Conversions|ToFloat(Integer) (* (+ _index 1) _returnvalue)))) (* (Math|Trig|Sin(Degrees) (Math|Conversions|ToFloat(Integer) (* (+ _index 1) _returnvalue))) (Variables|Default|GetRadius)) 0.0) (Math|Vector|MakeVector (* (Math|Trig|Sin(Degrees) (Math|Conversions|ToFloat(Integer) _returnvalue)) (* _returnvalue_2 -1.0)) (* (Math|Trig|Cos(Degrees) (Math|Conversions|ToFloat(Integer) (+ _index 1))) _returnvalue_2) 0.0) (Math|Vector|MakeVector (* (Math|Trig|Sin(Degrees) (Math|Conversions|ToFloat(Integer) _returnvalue)) (* _returnvalue_2 -1.0)) (* (Math|Trig|Cos(Degrees) (Math|Conversions|ToFloat(Integer) (+ _index 1))) _returnvalue_2) 0.0) true :!class /Script/Engine.SplineMeshComponent)))